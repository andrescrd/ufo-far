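; EnemyCow is a wandering cow that can be abducted and destroyed.
; Tick drives Move through a DoOnce, sending the cow by AI MoveTo to a random navigable point around it and re-arming after a delay while CanMove holds.
; StartAbduction enables physics on the capsule, and EndAbduction disables it and resets the rotation.
; Destroy removes the actor and prints a moo.
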(event Custom|Move
  ;[1 1 1] Move Cow
  (Utilities|FlowControl|DoOnce false :!label _label
    (:Completed
      (if (Variables|Default|GetCanMove)
        (Utilities|FlowControl|Sequence
          (:then_0
            (bind _newparam (CallFunction|GetNewLocation))
            (AI|AIMoveTo self _newparam 0 5.0 false))
          (:then_1
            (Utilities|FlowControl|Delay 5.0)
            (goto _label Reset)))))))

(event Custom|Destroy
  ;[1 1 1] Destroy Cow
  (Actor|DestroyActor)
  (Development|PrintString "MUUUUUUUU"))

(event Custom|StartAbduction
  ;[1 1 1] Abduction beahviour
  (Physics|SetSimulatePhysics (Variables|Collision|GetCapsuleComponent) true))

(event Custom|EndAbduction
  ;[1 1 1] Abduction beahviour
  (Physics|SetSimulatePhysics (Variables|Collision|GetCapsuleComponent) false)
  (Transformation|SetActorRotation (Math|Interpolation|RInterpTo (Transformation|GetActorRotation) "0, 0, 0" (Utilities|Time|GetWorldDeltaSeconds) 0.0)))

(event EventTick
  (params (DeltaSeconds :type Float%20%28single-precision%29))
  (CallFunction|Move))

(fn ConstructionScript)

(fn GetNewLocation
  (bind _randomlocation (Class|NavigationSystemV1|GetRandomLocationinNavigableRadius (Transformation|GetActorLocation) 9e+03 0 0))
  (return _randomlocation))