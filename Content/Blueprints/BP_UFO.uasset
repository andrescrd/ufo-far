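; Player-controlled UFO pawn that flies around and abducts BP_Abducted_Base actors with a tractor beam.
; Tick adds camera-yaw-relative input to physics velocity, interpolates a pitch-clamped spring arm and look-at camera, and tilts the hull with movement.
; Holding left mouse shows the beam light and pulls actors in AbductionTrigger toward the UFO's location scaled by BeamStrenght.
; Entering AbductionZone while beaming calls Abducted, updates AbductedActors and prints its count.
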(event OnComponentBeginOverlap(AbductionZone)
  (params (OverlappedComponent :type Primitive%20Component%20Object%20Reference) (OtherActor :type Actor%20Object%20Reference) (OtherComp :type Primitive%20Component%20Object%20Reference) (OtherBodyIndex :type Integer) (bFromSweep :type Boolean) (SweepResult :type Hit%20Result%20Structure%20%28by%20ref%29))
  ;[1 1 1] Hidde abducted actor
  (if (Variables|Default|GetBeam%20on)
    (bind _asbp_abducted_base (Utilities|Casting|CastToBP_Abducted_Base OtherActor))
    (Default|Abducted _asbp_abducted_base)
    (Utilities|Array|Add (Variables|Default|GetAbducted%20actors) 0)
    (Development|PrintString (Utilities|String|ToString(Integer) (Utilities|Array|Length (Variables|Default|GetAbducted%20actors))))))

(event EventTick
  (params (DeltaSeconds :type Float%20%28single-precision%29))
  (bind _camera (Variables|Default|GetCamera))
  (bind _abduction_trigger (Variables|Default|GetAbduction%20Trigger))
  (bind _springarm (Variables|Default|GetSpringArm))
  (bind _camera_speed (Variables|Default|GetCamera%20speed))
  (bind _returnvalue (Transformation|GetWorldRotation _springarm))
  (bind _overlappingactors (Collision|GetOverlappingActors _abduction_trigger "/Game/Blueprints/BP_Abducted_Base.BP_Abducted_Base_C" :!class /Script/Engine.PrimitiveComponent))
  (Variables|Default|SetDelta%20seconds DeltaSeconds)
  ;[1 1 1] Update Pawn Movement
  (Physics|SetPhysicsLinearVelocity (Variables|Default|GetBody) (+ (Transformation|GetVelocity) (* (* (Math|Vector|RotateVector (Math|Vector|MakeVector (Input|AxisValues|GetMoveForward) (Input|AxisValues|GetMoveRight) (Input|AxisValues|GetMoveUp)) (Math|Rotator|MakeRotator 0.0 0.0 (.yaw (Transformation|GetWorldRotation (Variables|Default|GetCamera))))) (Variables|Default|GetMovement%20speed)) (Variables|Default|GetDelta%20seconds))) false "None")
  ;[1 1 1] Update Camera Movement
  (Transformation|SetWorldRotation (Variables|Default|GetSpringArm) (Math|Interpolation|RInterpTo (Transformation|GetWorldRotation (Variables|Default|GetSpringArm)) (Math|Rotator|MakeRotator 0.0 (Math|Float|ClampAngle (+ (.pitch _returnvalue) (* (Input|AxisValues|GetLookUp) (* _camera_speed -1.0))) -45.0 85.0) (+ (.yaw _returnvalue) (* _camera_speed (Input|AxisValues|GetTurn)))) (Variables|Default|GetDelta%20seconds) 8.0) false false)
  ;[1 1 1] Update camera rotation
  (Transformation|SetWorldRotation (Variables|Default|GetCamera) (Math|Interpolation|RInterpTo (Transformation|GetWorldRotation _camera) (Math|Rotator|FindLookatRotation (Transformation|GetWorldLocation _camera) (Transformation|GetActorLocation)) (Variables|Default|GetDelta%20seconds) 2.0) false false)
  ;[1 1 1] Update Pawn Rotation
  (Transformation|SetActorRotation (Math|Interpolation|RInterpTo (Transformation|GetActorRotation) (Math|Rotator|MakeRotator (* (Input|AxisValues|GetMoveRight) 2e+01) (* (Input|AxisValues|GetMoveForward) -7.0) (.yaw (Math|Rotator|FindLookatRotation (Transformation|GetWorldLocation (Variables|Default|GetCamera)) (Transformation|GetActorLocation)))) (Variables|Default|GetDelta%20seconds) 4.0))
  ;[1 1 1] Abduction
  (if (Variables|Default|GetBeam%20on)
    (if (> (Utilities|Array|Length _overlappingactors) 0)
      (for _array_element _overlappingactors
        (bind _asbp_abducted_base (Utilities|Casting|CastToBP_Abducted_Base _array_element))
        (Transformation|SetActorLocation _asbp_abducted_base (Math|Interpolation|VInterpTo (Transformation|GetActorLocation _asbp_abducted_base) (* (Transformation|GetActorLocation) (Variables|Default|GetBeam%20Strenght)) (Variables|Default|GetDelta%20seconds) 5.0) false false)))))

(event Input|MouseEvents|LeftMouseButton
  (params (Key :type Key%20Structure))
  ;[1 1 1] Turn on light and  enable disable abduction
  (:Pressed
    (Variables|Default|SetBeam%20on true)
    (Rendering|SetVisibility (Variables|Default|GetAbductionLight) true false))
  (:Released
    (Variables|Default|SetBeam%20on false)
    (Rendering|SetVisibility (Variables|Default|GetAbductionLight) false false)))

(fn ConstructionScript)